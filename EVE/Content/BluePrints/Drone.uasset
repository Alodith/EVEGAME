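; Drone actor that fires a laser trace along its forward vector every tick, with a particle effect while active.
; With LookAt on, it picks the nearest TargetActor within a fixed radius and smoothly rotates toward it; otherwise it fires straight ahead.
; Hits pass ShootLaser to Destructible components and Conduits.
; Glass hits only store a reflection vector scaled by remaining range, and Cooldown counts down without gating anything.
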(event EventTick
  (params (DeltaSeconds :type Float%20%28single-precision%29))
  (bind _returnvalue (Transformation|GetActorLocation))
  (Components|Activation|SetActive (Variables|Default|GetParticleSystem) false false)
  (if (Variables|Default|GetLookAt)
    (Variables|Default|SetCooldown (- (Variables|Default|GetCooldown) DeltaSeconds))
    (if (Utilities|IsValid (Variables|Default|GetCurrentTarget))
      (Transformation|SetActorRotation (Math|Interpolation|RInterpTo (Transformation|GetActorRotation) (Math|Rotator|FindLookatRotation (Transformation|GetActorLocation) (Transformation|GetActorLocation (Variables|Default|GetCurrentTarget))) DeltaSeconds (Variables|Default|GetInterpSpeed)))
      (Components|Activation|SetActive (Variables|Default|GetParticleSystem) true false :!label _label)
      (bind (_outhit _returnvalue_2) (Collision|LineTraceByChannel _returnvalue (+ _returnvalue (* (Transformation|GetActorForwardVector) (Variables|Default|GetRange))) "TraceTypeQuery1" false 0 "ForOneFrame"))
      (Variables|Default|SetLastHit (.HitActor (Collision|BreakHitResult _outhit)))
      (Variables|Default|SetHitLoc (.ImpactPoint (Collision|BreakHitResult _outhit)))
      (if _returnvalue_2
        (if (== (Utilities|GetClass (.HitActor (Collision|BreakHitResult _outhit))) "/Game/BluePrints/Glass.Glass_C")
          (Variables|Default|SetLeftDist (* (Math|Vector|GetReflectionVector (Transformation|GetActorForwardVector) (.ImpactNormal (Collision|BreakHitResult _outhit))) (- (Variables|Default|GetRange) (.Distance (Collision|BreakHitResult _outhit))))))
        (if (Utilities|IsValid (Actor|GetComponentbyClass (.HitActor (Collision|BreakHitResult _outhit)) "/Game/BluePrints/Destructible.Destructible_C"))
          (Default|Hit (Actor|GetComponentbyClass (.HitActor (Collision|BreakHitResult _outhit)) "/Game/BluePrints/Destructible.Destructible_C") (Variables|Default|GetShootLaser)))
        (if (== (Utilities|GetClass (.HitActor (Collision|BreakHitResult _outhit))) "/Game/BluePrints/Conduit.Conduit_C")
          (bind _asconduit (Utilities|Casting|CastToConduit (.HitActor (Collision|BreakHitResult _outhit))))
          (Variables|/Game/BluePrints/Conduit.Conduit_C|SetOnLaser _asconduit (Variables|Default|GetShootLaser))))
      (else
        (bind _outactors (Actor|GetAllActorsOfClass (Variables|Default|GetTargetActor)))
        (if (Utilities|Array|IsValidIndex _outactors)
          (Variables|Default|SetTempTarget (Utilities|Array|Get(acopy) _outactors))
          (for _array_element _outactors
            (if (< (Transformation|GetDistanceTo _array_element) (Transformation|GetDistanceTo (Variables|Default|GetTempTarget)))
              (Variables|Default|SetTempTarget _array_element)))
          (if (< (Transformation|GetDistanceTo (Variables|Default|GetTempTarget)) 1e+03)
            (Variables|Default|SetCurrentTarget (Variables|Default|GetTempTarget))))))
    (else
      (goto _label))))

(fn ConstructionScript)