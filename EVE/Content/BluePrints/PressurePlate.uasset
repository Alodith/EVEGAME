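; Pressure plate Blueprint that activates while a weighted actor rests in its trigger.
; Each tick it clears its pressed state, then scans the Trigger's overlapping actors for a "Weighted" tag, polling rather than using overlap events.
; The result is written to the Activator's Activated flag every tick, so activation drops as soon as no tagged actor overlaps.
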(event EventTick
  (params (DeltaSeconds :type Float%20%28single-precision%29))
  (bind _trigger (Variables|Default|GetTrigger))
  (bind _overlappingactors (Collision|GetOverlappingActors _trigger "/Script/Engine.Actor" :!class /Script/Engine.PrimitiveComponent))
  (Variables|Default|SetPressured false)
  (if (> (Utilities|Array|Length _overlappingactors) 0)
    (bind _array_element (Utilities|Array|ForEachLoopwithBreak _overlappingactors :!label _label)
      (:LoopBody
        (bind _array_element_2 (Utilities|Array|ForEachLoopwithBreak (Variables|/Script/Engine.Actor|GetTags _array_element))
          (:LoopBody
            (if (Utilities|Name|Equal(Name) _array_element_2 "Weighted")
              (Variables|Default|SetPressured true)
              (goto _label Break)))))
      (:Completed
        (Variables|/Game/BluePrints/Activator.Activator_C|SetActivated (Variables|Default|GetActivator) (Variables|Default|GetPressured) :!label _label_2)))
    (else
      (goto _label_2))))

(fn ConstructionScript)