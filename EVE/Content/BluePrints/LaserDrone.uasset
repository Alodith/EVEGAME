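; Laser drone that traces a laser each tick, passing its ShootLaser value to Destructible components and Conduit actors it hits.
; A loop repeats line traces while a remaining distance vector is non-zero, ignoring the previous hit actor.
; Glass hits redirect the trace with a reflection vector scaled by hit distance, while other hits end it.
; The particle beam's target is then set to the last stored hit location.
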(event EventTick
  (params (DeltaSeconds :type Float%20%28single-precision%29))
  (|CallParentFunction DeltaSeconds)
  (while (Math|Vector|NotEqual(Vector) (Variables|Default|GetLeftDist) "0, 0, 0" 1.0)
    (bind (_outhit _returnvalue) (Collision|LineTraceByChannel (Variables|Default|GetHitLoc) (+ (Variables|Default|GetHitLoc) (Variables|Default|GetLeftDist)) "TraceTypeQuery1" false (Utilities|Array|MakeArray (Variables|Default|GetLastHit)) "ForOneFrame"))
    (if _returnvalue
      (if (Utilities|IsValid (Actor|GetComponentbyClass (.HitActor (Collision|BreakHitResult _outhit)) "/Game/BluePrints/Destructible.Destructible_C"))
        (Default|Hit (Actor|GetComponentbyClass (.HitActor (Collision|BreakHitResult _outhit)) "/Game/BluePrints/Destructible.Destructible_C") (Variables|Default|GetShootLaser))))
    (Variables|Default|SetLastHit (.HitActor (Collision|BreakHitResult _outhit)))
    (if (!= (Utilities|GetClass (.HitActor (Collision|BreakHitResult _outhit))) "/Game/BluePrints/Glass.Glass_C")
      (Variables|Default|SetLeftDist "0, 0, 0")
      (else
        (Variables|Default|SetHitLoc (.ImpactPoint (Collision|BreakHitResult _outhit)))
        (Variables|Default|SetLeftDist (* (* (Math|Vector|GetReflectionVector (+ (Variables|Default|GetHitLoc) (Variables|Default|GetLeftDist)) (.ImpactNormal (Collision|BreakHitResult _outhit))) (.Distance (Collision|BreakHitResult _outhit))) -1))))
    (if (== (Utilities|GetClass (.HitActor (Collision|BreakHitResult _outhit))) "/Game/BluePrints/Conduit.Conduit_C")
      (bind _asconduit (Utilities|Casting|CastToConduit (.HitActor (Collision|BreakHitResult _outhit))))
      (Variables|/Game/BluePrints/Conduit.Conduit_C|SetOnLaser _asconduit (Variables|Default|GetShootLaser))))
  (Class|ParticleSystemComponent|SetBeamTargetPoint (Variables|Default|GetParticleSystem) 0 (Variables|Default|GetHitLoc)))

(fn ConstructionScript
  (|CallParentFunction))