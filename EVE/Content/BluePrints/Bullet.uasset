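; Bullet projectile that flies straight along its forward vector and destroys itself on impact, passing through actors tagged "Drone".
; Each Tick checks the HitBox's overlapping actors and destroys the bullet if any lacks that tag, otherwise moving it at constant speed without sweep.
; A HitBox component hit event also destroys it, with no tag check.
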(event OnComponentHit(HitBox)
  (params (HitComponent :type Primitive%20Component%20Object%20Reference) (OtherActor :type Actor%20Object%20Reference) (OtherComp :type Primitive%20Component%20Object%20Reference) (NormalImpulse :type Vector :default "0, 0, 0") (Hit :type Hit%20Result%20Structure%20%28by%20ref%29))
  (if true
    (Actor|DestroyActor)))

(event EventTick
  (params (DeltaSeconds :type Float%20%28single-precision%29))
  (bind _hitbox (Variables|Default|GetHitBox))
  (bind _overlappingactors (Collision|GetOverlappingActors _hitbox 0 :!class /Script/Engine.PrimitiveComponent))
  (if (> (Utilities|Array|Length _overlappingactors) 0)
    (Variables|Default|SetHit false)
    (bind _array_element (Utilities|Array|ForEachLoopwithBreak _overlappingactors :!label _label)
      (:LoopBody
        (if (not (Actor|ActorHasTag _array_element "Drone"))
          (Variables|Default|SetHit true)
          (goto _label Break)))
      (:Completed
        (if (Variables|Default|GetHit)
          (Actor|DestroyActor)
          (else
            (Transformation|SetActorLocation (+ (Transformation|GetActorLocation) (* (* (Transformation|GetActorForwardVector) 2.5e+03) DeltaSeconds)) false false :!label _label_2)))))
    (else
      (goto _label_2))))

(fn ConstructionScript)