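; Alien barnacle actor that latches onto the first component to enter its trigger sphere and holds it relative to itself.
; On overlap, if nothing is held, a PhysicsHandle grabs the component and stores its offset from the actor.
; Tick keeps the handle target at that offset, so the held component follows the barnacle.
; When destroyed, it calls Hit on the held owner's Destructible component, if present.
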(event OnComponentBeginOverlap(TriggerSphere)
  (params (OverlappedComponent :type Primitive%20Component%20Object%20Reference) (OtherActor :type Actor%20Object%20Reference) (OtherComp :type Primitive%20Component%20Object%20Reference) (OtherBodyIndex :type Integer) (bFromSweep :type Boolean) (SweepResult :type Hit%20Result%20Structure%20%28by%20ref%29))
  (bind _returnvalue (Transformation|GetWorldLocation OtherComp))
  (bind _physicshandle (Variables|Default|GetPhysicsHandle))
  (if (not (Utilities|IsValid (Class|PhysicsHandleComponent|GetGrabbedComponent _physicshandle)))
    (Physics|Components|PhysicsHandle|GrabComponentatLocationwithRotation _physicshandle OtherComp "None" _returnvalue (Transformation|GetWorldRotation OtherComp))
    (Variables|Default|SetTargetLocation (- _returnvalue (Transformation|GetActorLocation)))))

(event EventTick
  (params (DeltaSeconds :type Float%20%28single-precision%29))
  (Physics|Components|PhysicsHandle|SetTargetLocation (Variables|Default|GetPhysicsHandle) (+ (Transformation|GetActorLocation) (Variables|Default|GetTargetLocation))))

(event EventDestroyed
  (bind _physicshandle (Variables|Default|GetPhysicsHandle))
  (bind _returnvalue (Class|PhysicsHandleComponent|GetGrabbedComponent _physicshandle))
  (bind _returnvalue_2 (Components|GetOwner _returnvalue))
  (bind _returnvalue_3 (Actor|GetComponentbyClass _returnvalue_2 "/Game/BluePrints/Destructible.Destructible_C"))
  (if (Utilities|IsValid _returnvalue)
    (if (Utilities|IsValid _returnvalue_3)
      (Default|Hit _returnvalue_3 false))))

(fn ConstructionScript
  (|CallParentFunction))