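; Activator is a Blueprint that mirrors its Activated state onto an Activatable component of another actor in the level.
; On BeginPlay it finds the first actor with AttachedTag and caches that actor's Activatable component.
; Every Tick it copies its own Activated flag to that component while the reference is valid.
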(event EventBeginPlay
  ;[1 1 1] Activate attached
  (bind _outactors (Actor|GetAllActorswithTag (Variables|Default|GetAttachedTag)))
  (Variables|Default|SetAttached (Actor|GetComponentbyClass (Utilities|Array|Get(acopy) _outactors) "/Game/BluePrints/Activatable.Activatable_C")))

(event EventTick
  (params (DeltaSeconds :type Float%20%28single-precision%29))
  (bind _attached (Variables|Default|GetAttached))
  ;[1 1 1] Activate attached
  (if (Utilities|IsValid _attached)
    (Variables|/Game/BluePrints/Activatable.Activatable_C|SetActivated _attached (Variables|Default|GetActivated))))